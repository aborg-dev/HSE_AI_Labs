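; Ball Blueprint for a Pong game that reports its state to the game mode.
; Every tick it writes its location and velocity to Pong_GameMode_BP as 2D vectors built from the X and Z axes.
; The sphere's hit event casts the other actor to Paddle_BP but does nothing further.
; Two ping-pong sound nodes are present but unconnected, so they never play.
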(event OnComponentHit(Sphere_Shape)
  (params (HitComponent :type Primitive%20Component%20Object%20Reference) (OtherActor :type Actor%20Object%20Reference) (OtherComp :type Primitive%20Component%20Object%20Reference) (NormalImpulse :type Vector :default "0, 0, 0") (Hit :type Hit%20Result%20Structure%20%28by%20ref%29))
  (Utilities|Casting|CastToPaddle_BP OtherActor))

(event EventTick
  (params (DeltaSeconds :type Float%20%28single-precision%29))
  (bind _returnvalue (Transformation|GetVelocity))
  (bind _returnvalue_2 (Transformation|GetActorLocation))
  (bind (_x _y _z) (Math|Vector|BreakVector _returnvalue_2))
  (bind (_x_2 _y_2 _z_2) (Math|Vector|BreakVector _returnvalue))
  (bind _aspong_game_mode_bp (Utilities|Casting|CastToPong_GameMode_BP (Game|GetGameMode)))
  (Variables|/Script/PongGame.Pong_GameMode|SetBallPosition _aspong_game_mode_bp (Math|Vector2D|MakeVector2D _x _z))
  (Variables|/Script/PongGame.Pong_GameMode|SetBallSpeed _aspong_game_mode_bp (Math|Vector2D|MakeVector2D _x_2 _z_2)))

(fn ConstructionScript)