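; Paddle Blueprint for a Pong game, controlled either as the player or as the AI opponent.
; On Tick, a player paddle moves vertically by its movement direction and speed, with sweep collision.
; An AI paddle gets the ball from the Pong game mode and follows its height at constant speed, only while the ball travels toward negative X.
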(event EventTick
  (params (DeltaSeconds :type Float%20%28single-precision%29))
  (bind _returnvalue (Transformation|GetActorLocation))
  (if (Variables|Default|GetIsPlayer)
    (Transformation|AddActorWorldOffset (* "0, 0,1.000000" (* (Variables|Default|GetMovementDirection) (Utilities|Time|GetWorldDeltaSeconds) (Variables|Default|GetPaddleSpeed))) true)
    (else
      (bind _aspong_game_mode_bp (Utilities|Casting|CastToPong_GameMode_BP (Variables|Default|GetGameMode)))
      (Utilities|IsValid (Variables|/Game/Blueprints/Pong_GameMode_BP.Pong_GameMode_BP_C|GetBall_Ref _aspong_game_mode_bp)
        (:Is%20Valid
          (Math|Float|CompareFloat (.x (Transformation|GetVelocity (Variables|/Game/Blueprints/Pong_GameMode_BP.Pong_GameMode_BP_C|GetBall_Ref _aspong_game_mode_bp))) 0.0
            (:<
              (Transformation|SetActorLocation (Math|Interpolation|VInterptoConstant (Transformation|GetActorLocation) (Math|Vector|MakeVector (.x _returnvalue) (.y _returnvalue) (.z (Transformation|GetWorldLocation (Variables|/Game/Blueprints/Ball_BP.Ball_BP_C|GetSphere_Shape (Variables|/Game/Blueprints/Pong_GameMode_BP.Pong_GameMode_BP_C|GetBall_Ref _aspong_game_mode_bp))))) (Utilities|Time|GetWorldDeltaSeconds) (Variables|Default|GetPaddleSpeed)) true false))))))))

(event EventBeginPlay
  (bind _aspong_game_mode_bp (Utilities|Casting|CastToPong_GameMode_BP (Game|GetGameMode)))
  (Variables|Default|SetGameMode _aspong_game_mode_bp))

(fn ConstructionScript)