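; Pong paddle actor that serves as either the player's paddle or the AI opponent, selected by an IsPlayer flag.
; Each tick, a player paddle moves vertically with a swept offset driven by the VerticalMovementAxis input and PaddleSpeed.
; The AI paddle reads the ball from Pong_GameMode_BP and, only while it travels toward negative X, tracks its height using constant-speed interpolation with sweep.
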(event EventTick
  (params (DeltaSeconds :type Float%20%28single-precision%29))
  (bind _returnvalue (Transformation|GetActorLocation))
  (bind _gamemode (Variables|Default|GetGameMode))
  (bind _ball_ref (Variables|/Game/Blueprints/Pong_GameMode_BP.Pong_GameMode_BP_C|GetBall_Ref _gamemode))
  (if (Variables|Default|GetIsPlayer)
    (Transformation|AddActorWorldOffset (* "0, 0,1.000000" (* (Input|AxisValues|GetVerticalMovementAxis) (Utilities|Time|GetWorldDeltaSeconds) (Variables|Default|GetPaddleSpeed))) true)
    (else
      (Utilities|IsValid _ball_ref
        (:Is%20Valid
          (Math|Float|CompareFloat (.x (Transformation|GetVelocity _ball_ref)) 0.0
            (:<
              (Transformation|SetActorLocation (Math|Interpolation|VInterptoConstant (Transformation|GetActorLocation) (Math|Vector|MakeVector (.x _returnvalue) (.y _returnvalue) (.z (Transformation|GetWorldLocation (Variables|/Game/Blueprints/Ball_BP.Ball_BP_C|GetSphere_Shape _ball_ref)))) (Utilities|Time|GetWorldDeltaSeconds) (Variables|Default|GetPaddleSpeed)) true false))))))))

(event EventBeginPlay
  (bind _aspong_game_mode_bp (Utilities|Casting|CastToPong_GameMode_BP (Game|GetGameMode)))
  (Variables|Default|SetGameMode _aspong_game_mode_bp))

(fn ConstructionScript)